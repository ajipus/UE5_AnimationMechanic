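; Enemy AI character that wanders, chases the player on sight and shoots with a rifle.
; After a short delay it patrols by looping AI MoveTo to random nearby reachable points; PawnSensing spotting BP_PlayerTask4 triggers a chase.
; Reaching the target fires one montage-backed debug line trace from the muzzle that applies damage, with a brief DoOnce cooldown.
; Damage lowers health, and death only ragdolls the mesh without stopping the AI logic.
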(event OnSeePawn(PawnSensing)
  (params (Pawn :type Pawn%20Object%20Reference))
  ;[1 1 1] Sensing
  (bind _asbp_player_task_4 (Utilities|Casting|CastToBP_PlayerTask4 Pawn))
  (CallFunction|ChasePlayer _asbp_player_task_4))

(event Custom|Patrol
  ;[1 1 1] Patrol
  (AI|AIMoveTo self (.RandomLocation (AI|Navigation|GetRandomReachablePointinRadius (Transformation|GetActorLocation) 3e+02 0 0)) 0 5.0 false
    (:OnSuccess
      _)
    (:OnFail
      _))
  (CallFunction|Patrol))

(event Custom|Fire
  (bind _rifle (Variables|Default|GetRifle))
  (bind _returnvalue (Transformation|GetSocketTransform _rifle "Muzzle" "RTS_World"))
  ;[1 1 1] Fire
  (Utilities|FlowControl|DoOnce false :!label _label
    (:Completed
      (Utilities|FlowControl|Sequence
        (:then_0
          (Animation|Montage|PlayMontage (Variables|Character|GetMesh) "/Game/AnimationShooter/AM_Fire.AM_Fire"
            (:then
              (bind (_outhit _returnvalue_2) (Collision|LineTraceByChannel (.location _returnvalue) (+ (.location _returnvalue) (* (Math|Vector|GetRightVector (Variables|Character|GetMesh)) 3e+03)) "TraceTypeQuery1" false 0 "ForDuration"))
              (if _returnvalue_2
                (Development|PrintString (Utilities|GetDisplayName (.HitActor (Collision|BreakHitResult _outhit))))
                (Game|Damage|ApplyDamage (.HitActor (Collision|BreakHitResult _outhit)) 1e+01 0 0)))))
        (:then_1
          (Utilities|FlowControl|Delay 0.2)
          (goto _label Reset))))))

(event Custom|Chase%20Player
  (params (TargetActor :type Actor%20Object%20Reference))
  ;[1 1 1] ChasePlayer
  (AI|AIMoveTo self "0, 0, 0" TargetActor 3e+02 false
    (:OnSuccess
      (CallFunction|Fire))))

(event EventBeginPlay
  (Utilities|FlowControl|Delay 2.0)
  (CallFunction|Patrol))

(event Collision|EventActorBeginOverlap
  (params (OtherActor :type Actor%20Object%20Reference)))

(event EventTick
  (params (DeltaSeconds :type Float%20%28single-precision%29)))

(event Game|Damage|EventAnyDamage
  (params (Damage :type Float%20%28single-precision%29) (DamageType :type Damage%20Type%20Object%20Reference) (InstigatedBy :type Controller%20Object%20Reference) (DamageCauser :type Actor%20Object%20Reference))
  ;[1 1 1] Damage
  (if (not (Variables|Default|GetIsDead))
    (Variables|Default|SetCurrentHealth (- (Variables|Default|GetCurrentHealth) Damage))
    (Variables|Default|SetIsDead (<= (Variables|Default|GetCurrentHealth) 0.0))
    (Development|PrintString (Utilities|String|ToString(Float) (Variables|Default|GetCurrentHealth)))
    (if (Variables|Default|GetIsDead)
      (Physics|SetSimulatePhysics (Variables|Character|GetMesh) true))))

(fn ConstructionScript)